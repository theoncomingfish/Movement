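; ProbeEffect_BP is a temporary probe effect actor that marks an area for twenty seconds, then clears stencil-based marking on nearby AI characters.
; On BeginPlay it draws a debug sphere at its location and waits out the same duration.
; It then sets the mesh custom depth stencil to zero on every AI_Character within the sphere's radius and destroys itself.
; The stencil value is only reset here, never raised.
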(event EventBeginPlay
  (bind _output_get (Variables|Default|SetLocation (Transformation|GetActorLocation)))
  (Rendering|Debug|DrawDebugSphere _output_get 1e+03 12 "(R=0.245767,G=1.000000,B=0.057882,A=1.000000)" 2e+01)
  (Utilities|FlowControl|Delay 2e+01)
  (bind _outactors (Actor|GetAllActorsOfClass "/Game/Raynes/AI_Character.AI_Character_C"))
  (for _array_element _outactors
    (if (<= (Transformation|GetDistanceTo _array_element self) 1e+03)
      (bind _asai_character (Utilities|Casting|CastToAI_Character _array_element))
      (Rendering|SetCustomDepthStencilValue (Variables|/Script/Engine.Character|GetMesh _asai_character) 0)))
  (Actor|DestroyActor))

(fn ConstructionScript)