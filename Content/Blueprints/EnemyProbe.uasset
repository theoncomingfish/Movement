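; EnemyProbe is a moving probe actor that flies in a straight line and spawns an EnemyProbeEffect when it overlaps something.
; Tick sets Direction toward End while it is zero, then moves the probe by Speed and delta time without sweeping.
; Overlaps ignore AI-tagged actors, probes and effects; others spawn the effect offset 1000 units along the away vector's X/Y, with Z doubled, then destroy the probe.
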(event Collision|EventActorBeginOverlap
  (params (OtherActor :type Actor%20Object%20Reference))
  (bind _returnvalue (Utilities|GetClass OtherActor))
  (bind _returnvalue_2 (Transformation|GetActorLocation OtherActor))
  (bind _returnvalue_3 (Transformation|GetActorTransform))
  (bind (_location _rotation _scale) (Math|Transform|BreakTransform _returnvalue_3))
  (bind _returnvalue_4 (Math|Vector|GetUnitDirection(Vector) _returnvalue_2 _location))
  (bind _returnvalue_5 (Math|Vector|Normalize _returnvalue_4))
  (bind _returnvalue_6 (* _returnvalue_5 1e+03))
  (bind (_x _y) (Math|Vector|BreakVector _returnvalue_6))
  (if (and (and (not (Actor|ActorHasTag OtherActor "AI")) (!= _returnvalue "EnemyProbe_C")) (!= _returnvalue "/Game/Blueprints/EnemyProbeEffect.EnemyProbeEffect_C"))
    (Game|SpawnActorfromClass "/Game/Blueprints/EnemyProbeEffect.EnemyProbeEffect_C" (Math|Transform|MakeTransform (+ (Math|Vector|MakeVector _x _y (.Z (Math|Vector|BreakVector _location))) _location) _rotation _scale) "AlwaysSpawn" (Components|GetOwner) (Game|GetInstigator))
    (Actor|DestroyActor)))

(event EventTick
  (params (DeltaSeconds :type Float%20%28single-precision%29))
  (bind _returnvalue (Transformation|GetActorTransform))
  (bind (_location _rotation _scale) (Math|Transform|BreakTransform _returnvalue))
  (if (Math|Vector|NotEqual(Vector) (Variables|Default|GetDirection) "0, 0, 0" 0.0)
    _
    (else
      (Variables|Default|SetDirection (Math|Vector|GetUnitDirection(Vector) (Transformation|GetActorLocation) (Variables|Default|Getend)))))
  (Transformation|SetActorTransform (Math|Transform|MakeTransform (+ (* (Variables|Default|GetDirection) (* (Utilities|Time|GetWorldDeltaSeconds) (Variables|Default|GetSpeed))) _location) _rotation _scale)))

(fn ConstructionScript)