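; Decoy actor with a skeletal mesh that travels in a straight line toward an End point, then removes itself.
; It briefly shows one material on spawn before switching to a second.
; Tick moves it by Speed and delta time without sweeping, restoring the first material shortly before destroying it on arrival.
; When remaining lifespan runs low, Tick stops movement and applies that first material instead.
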(event EventBeginPlay
  (bind _returnvalue (Transformation|GetActorTransform))
  (bind (_location _rotation _scale) (Math|Transform|BreakTransform _returnvalue))
  (Rendering|Material|SetMaterial (Variables|Default|GetSkeletalMesh) 0 (Variables|Default|Getmat))
  (Utilities|FlowControl|Delay 0.3)
  (Rendering|Material|SetMaterial (Variables|Default|GetSkeletalMesh) 0 (Variables|Default|Getmat2))
  (Variables|Default|SetDirection (Math|Vector|GetUnitDirection(Vector) (Transformation|GetActorLocation) (Variables|Default|Getend)))
  (Transformation|SetActorTransform (Math|Transform|MakeTransform (+ (* (Variables|Default|GetDirection) (* (Utilities|Time|GetWorldDeltaSeconds) (Variables|Default|GetSpeed))) _location) _rotation _scale))
  (if (Math|Vector|Equal(Vector) (Transformation|GetActorLocation) (Variables|Default|Getend self) 5.0)
    (Rendering|Material|SetMaterial (Variables|Default|GetSkeletalMesh) 0 (Variables|Default|Getmat))
    (Utilities|FlowControl|Delay 0.3)
    (Actor|DestroyActor)))

(event EventTick
  (params (DeltaSeconds :type Float%20%28single-precision%29))
  (bind _returnvalue (Transformation|GetActorTransform))
  (bind (_location _rotation _scale) (Math|Transform|BreakTransform _returnvalue))
  (if (>= (Actor|GetLifeSpan) 0.3)
    (Variables|Default|SetDirection (Math|Vector|GetUnitDirection(Vector) (Transformation|GetActorLocation) (Variables|Default|Getend)))
    (Transformation|SetActorTransform (Math|Transform|MakeTransform (+ (* (Variables|Default|GetDirection) (* (Utilities|Time|GetWorldDeltaSeconds) (Variables|Default|GetSpeed))) _location) _rotation _scale))
    (if (Math|Vector|Equal(Vector) (Transformation|GetActorLocation) (Variables|Default|Getend self) 5.0)
      (Rendering|Material|SetMaterial (Variables|Default|GetSkeletalMesh) 0 (Variables|Default|Getmat))
      (Utilities|FlowControl|Delay 0.3)
      (Actor|DestroyActor))
    (else
      (Rendering|Material|SetMaterial (Variables|Default|GetSkeletalMesh) 0 (Variables|Default|Getmat)))))

(fn ConstructionScript)