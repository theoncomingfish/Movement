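; Objective_BP is a spinning collectible objective that increments the player character's Collectibles count when MovementCharacter_BP overlaps it.
; On BeginPlay it caches the character and all PotentialObjectiveSpawns_BP actors, identifying its current spawn by matching transforms.
; On first overlap it picks random spawn points until one differs from the current, spawns a fresh Objective_BP there and destroys itself, with debug prints of locations.
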(event EventBeginPlay
  (Development|PrintString (Utilities|String|ToString(Vector) (Transformation|GetActorLocation)) true true "(R=0.000000,G=0.660000,B=1.000000,A=1.000000)" 5.0)
  (bind _outactors (Actor|GetAllActorsOfClass "/Game/Blueprints/MovementCharacter_BP.MovementCharacter_BP_C"))
  (for _array_element _outactors
    (Variables|Default|SetMovementCharacter _array_element))
  (bind _outactors_2 (Actor|GetAllActorsOfClass "/Game/Blueprints/PotentialObjectiveSpawns_BP.PotentialObjectiveSpawns_BP_C"))
  (bind _output_get (Variables|Default|SetSpawnLocations _outactors_2))
  (for _array_element_2 _output_get
    (if (== (Transformation|GetActorTransform _array_element_2) (Transformation|GetActorTransform))
      (Variables|Default|SetCurrentSpawn _array_element_2)
      (Variables|Default|SetNextSpawn (Variables|Default|GetCurrentSpawn)))))

(event Collision|EventActorBeginOverlap
  (params (OtherActor :type Actor%20Object%20Reference))
  (bind _spawnlocations (Variables|Default|GetSpawnLocations))
  (bind _movementcharacter (Variables|Default|GetMovementCharacter))
  (if (== OtherActor (Variables|Default|GetMovementCharacter))
    (if (not (Variables|Default|Gettriggered))
      (Variables|Default|Settriggered true)
      (Development|PrintString (Utilities|String|ToString(Vector) (Transformation|GetActorLocation)) true false "(R=0.763667,G=0.166146,B=1.000000,A=1.000000)" 5.0)
      (while (== (Variables|Default|GetCurrentSpawn) (Variables|Default|GetNextSpawn))
        (Variables|Default|SetNextSpawn (Utilities|Array|Get(acopy) _spawnlocations (Math|Random|RandomInteger (Utilities|Array|Length _spawnlocations)))))
      (Game|SpawnActorfromClass "Objective_BP_C" (Transformation|GetActorTransform (Variables|Default|GetNextSpawn)) "AlwaysSpawn" 0 (Variables|Default|GetInstigator))
      (Development|PrintString (Utilities|String|ToString(Vector) (Transformation|GetActorLocation (Variables|Default|GetNextSpawn))) true true "(R=0.040000,G=1.000000,B=0.138874,A=1.000000)" 5.0)
      (bind _result (Math|Integer|IncrementInt (Variables|/Game/Blueprints/MovementCharacter_BP.MovementCharacter_BP_C|GetCollectibles _movementcharacter))
        (:%20%20
          (Variables|/Game/Blueprints/MovementCharacter_BP.MovementCharacter_BP_C|SetCollectibles _movementcharacter _result)
          (Actor|DestroyActor))))))

(event EventTick
  (params (DeltaSeconds :type Float%20%28single-precision%29))
  (Transformation|AddLocalRotation (Variables|Default|GetSphere) "0.100000,0.100000,0.100000" false false))

(fn ConstructionScript)