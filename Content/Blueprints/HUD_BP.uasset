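; HUD Blueprint that shows the player's collectible count as large cyan text near the top middle of the screen.
; Each DrawHUD call finds every MovementCharacter_BP actor, stores it in CharacterRef and draws its Collectibles value at half the screen width.
; The actor lookup repeats every frame rather than being cached.
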(event EventBeginPlay)

(event EventDrawHUD
  (params (SizeX :type Integer) (SizeY :type Integer))
  (bind _outactors (Actor|GetAllActorsOfClass "/Game/Blueprints/MovementCharacter_BP.MovementCharacter_BP_C"))
  (for _array_element _outactors
    (Variables|Default|SetCharacterRef _array_element)
    (HUD|DrawText (Utilities|String|ToString(Integer) (Variables|/Game/Blueprints/MovementCharacter_BP.MovementCharacter_BP_C|GetCollectibles (Variables|Default|GetCharacterRef))) "(R=0.228041,G=1.000000,B=0.960192,A=1.000000)" (Math|Conversions|ToFloat(Integer) (/ SizeX 2)) 0.0 0 5.0 false)))

(event EventTick
  (params (DeltaSeconds :type Float%20%28single-precision%29)))

(fn ConstructionScript)