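; EnemyProbeEffect is a timed effect actor that marks an AI_Character_Probe owner as probed for a limited time.
; On BeginPlay it records its location, waits 20 seconds, then clears the owner's Probed flag and destroys itself; destruction only happens if the owner cast succeeds.
; A ChangeMaterial function toggles Sphere1 between two materials, though nothing in this file calls it.
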(event EventBeginPlay
  (Variables|Default|SetLocation (Transformation|GetActorLocation))
  (Utilities|FlowControl|Delay 2e+01)
  (bind _asai_character_probe (Utilities|Casting|CastToAI_Character_Probe (Components|GetOwner)))
  (Variables|/Game/Raynes/AI_Character_Probe.AI_Character_Probe_C|SetProbed _asai_character_probe false)
  (Actor|DestroyActor))

(fn ConstructionScript)

(fn ChangeMaterial
  (if (== (Rendering|Material|GetMaterial (Variables|Default|GetSphere1) 0) (Variables|Default|GetMat1))
    (Rendering|Material|SetMaterial (Variables|Default|GetSphere1) 0 (Variables|Default|GetMat2))
    (else
      (Rendering|Material|SetMaterial (Variables|Default|GetSphere1) 0 (Variables|Default|GetMat1)))))