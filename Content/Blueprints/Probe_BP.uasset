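; Probe projectile that tags AI it touches or spawns a ProbeEffect_BP when it hits something else.
; Tick moves it without sweeping, at Speed along a direction set toward End whenever Direction is zero.
; Overlapping an AI-tagged AI_Character or AI_Character_Radar sets Tagged and expires the probe.
; Other overlaps, except the player character, probes and effects, spawn the effect offset away from that actor and destroy the probe.
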(event Collision|EventActorBeginOverlap
  (params (OtherActor :type Actor%20Object%20Reference))
  (bind _returnvalue (Utilities|GetClass OtherActor))
  (bind _returnvalue_2 (Transformation|GetActorTransform OtherActor))
  (bind _returnvalue_3 (Transformation|GetActorTransform))
  (bind _location (Math|Transform|BreakTransform _returnvalue_2))
  (bind (_location_2 _rotation _scale) (Math|Transform|BreakTransform _returnvalue_3))
  (bind _returnvalue_4 (Math|Vector|GetUnitDirection(Vector) _location _location_2))
  (bind _returnvalue_5 (Math|Vector|Normalize _returnvalue_4))
  (bind _returnvalue_6 (* _returnvalue_5 1e+03))
  (bind (_x _y) (Math|Vector|BreakVector _returnvalue_6))
  (if (Actor|ActorHasTag OtherActor "AI")
    (bind _asai_character (Utilities|Casting|CastToAI_Character OtherActor)
      (:then
        (Variables|/Game/Raynes/AI_Character.AI_Character_C|Settagged _asai_character true)
        (Actor|SetLifeSpan 0.01))
      (:CastFailed
        (bind _asai_character_radar (Utilities|Casting|CastToAI_Character_Radar OtherActor))
        (Variables|/Game/Raynes/AI_Character_Radar.AI_Character_Radar_C|Settagged _asai_character_radar true)
        (Actor|SetLifeSpan 0.01)))
    (elif (and (and (!= _returnvalue "/Game/Blueprints/MovementCharacter_BP.MovementCharacter_BP_C") (!= _returnvalue "Probe_BP_C")) (!= _returnvalue "/Game/Blueprints/ProbeEffect_BP.ProbeEffect_BP_C"))
      (Game|SpawnActorfromClass "/Game/Blueprints/ProbeEffect_BP.ProbeEffect_BP_C" (Math|Transform|MakeTransform (+ (Math|Vector|MakeVector _x _y (.Z (Math|Vector|BreakVector _location_2))) _location_2) _rotation _scale) "AlwaysSpawn" 0 (Game|GetInstigator))
      (Actor|DestroyActor))))

(event EventTick
  (params (DeltaSeconds :type Float%20%28single-precision%29))
  (bind _returnvalue (Transformation|GetActorTransform))
  (bind (_location _rotation _scale) (Math|Transform|BreakTransform _returnvalue))
  (if (Math|Vector|NotEqual(Vector) (Variables|Default|GetDirection) "0, 0, 0" 0.0)
    _
    (else
      (Variables|Default|SetDirection (Math|Vector|GetUnitDirection(Vector) (Transformation|GetActorLocation) (Variables|Default|Getend)))))
  (Transformation|SetActorTransform (Math|Transform|MakeTransform (+ (* (Variables|Default|GetDirection) (* (Utilities|Time|GetWorldDeltaSeconds) (Variables|Default|GetSpeed))) _location) _rotation _scale)))

(fn ConstructionScript)