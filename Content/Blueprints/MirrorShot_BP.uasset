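; MirrorShot_BP is a projectile that deploys a MirrorField_BP where it hits.
; From BeginPlay and every Tick, it moves its transform toward the End point at Speed, scaled by delta time, without sweeping.
; Overlapping any actor not of class MovementCharacter_BP spawns the field at the shot's transform and expires the shot almost immediately.
; DeployField also spawns the field and destroys the shot, but nothing in this file calls it.
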(event EventBeginPlay
  (bind _returnvalue (Transformation|GetActorTransform))
  (bind (_location _rotation _scale) (Math|Transform|BreakTransform _returnvalue))
  (Variables|Default|SetDirection (Math|Vector|GetUnitDirection(Vector) (Transformation|GetActorLocation) (Variables|Default|Getend)))
  (Transformation|SetActorTransform (Math|Transform|MakeTransform (+ (* (Variables|Default|GetDirection) (* (Utilities|Time|GetWorldDeltaSeconds) (Variables|Default|GetSpeed))) _location) _rotation _scale)))

(event Collision|EventActorBeginOverlap
  (params (OtherActor :type Actor%20Object%20Reference))
  (if (!= (Utilities|GetClass OtherActor) "/Game/Blueprints/MovementCharacter_BP.MovementCharacter_BP_C")
    (Game|SpawnActorfromClass "/Game/Blueprints/MirrorField_BP.MirrorField_BP_C" (Transformation|GetActorTransform) "AlwaysSpawn" 0 (Game|GetInstigator))
    (Actor|SetLifeSpan 0.01)))

(event EventTick
  (params (DeltaSeconds :type Float%20%28single-precision%29))
  (bind _returnvalue (Transformation|GetActorTransform))
  (bind (_location _rotation _scale) (Math|Transform|BreakTransform _returnvalue))
  (Variables|Default|SetDirection (Math|Vector|GetUnitDirection(Vector) (Transformation|GetActorLocation) (Variables|Default|Getend)))
  (Transformation|SetActorTransform (Math|Transform|MakeTransform (+ (* (Variables|Default|GetDirection) (* (Utilities|Time|GetWorldDeltaSeconds) (Variables|Default|GetSpeed))) _location) _rotation _scale)))

(fn ConstructionScript)

(fn DeployField
  (Game|SpawnActorfromClass "/Game/Blueprints/MirrorField_BP.MirrorField_BP_C" (Transformation|GetActorTransform) "Undefined" 0 (Game|GetInstigator))
  (Actor|DestroyActor))