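; Player craft character that manages engine effects, stealth lighting, gadget cooldowns and detection by probes.
; Tick runs mirror, decoy and probe cooldowns, switches engine sound and particles by MovementNumber, and cuts or dims effects and lights when Dark.
; Entering an enemy probe field writes the character's location and Sighted to that probe AI's blackboard and sets a custom-depth stencil highlight, cleared on exit.
; Deploy input triggers DeployField on every MirrorShot_BP.
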(event EventBeginPlay)

(event Collision|EventActorBeginOverlap
  (params (OtherActor :type Actor%20Object%20Reference))
  (bind _returnvalue (Utilities|GetClass OtherActor))
  (if (== _returnvalue "/Game/Blueprints/EnemyProbeEffect.EnemyProbeEffect_C")
    (bind _asenemy_probe_effect (Utilities|Casting|CastToEnemyProbeEffect OtherActor))
    (Default|ChangeMaterial _asenemy_probe_effect)
    (bind _asai_character_probe (Utilities|Casting|CastToAI_Character_Probe (Components|GetOwner _asenemy_probe_effect)))
    (bind _returnvalue_2 (AI|GetAIController _asai_character_probe))
    (AI|Components|Blackboard|SetValueasVector (AI|GetBlackboard _returnvalue_2) (Variables|Default|GetTargetLocation) (Transformation|GetActorLocation))
    (AI|Components|Blackboard|SetValueasBool (AI|GetBlackboard _returnvalue_2) (Variables|Default|GetSighted) true)
    (Rendering|SetCustomDepthStencilValue (Variables|Character|GetMesh) 253)
    (elif (== _returnvalue "/Game/Blueprints/ProbeEffect_BP.ProbeEffect_BP_C")
      (bind _asprobe_effect_bp (Utilities|Casting|CastToProbeEffect_BP OtherActor))
      (Default|ChangeMaterial _asprobe_effect_bp))))

(event Collision|EventActorEndOverlap
  (params (OtherActor :type Actor%20Object%20Reference))
  (bind _returnvalue (Utilities|GetClass OtherActor))
  (if (== _returnvalue "/Game/Blueprints/EnemyProbeEffect.EnemyProbeEffect_C")
    (Rendering|SetCustomDepthStencilValue (Variables|Character|GetMesh) 0)
    (bind _asenemy_probe_effect (Utilities|Casting|CastToEnemyProbeEffect OtherActor))
    (Default|ChangeMaterial _asenemy_probe_effect)
    (elif (== _returnvalue "/Game/Blueprints/ProbeEffect_BP.ProbeEffect_BP_C")
      (bind _asprobe_effect_bp (Utilities|Casting|CastToProbeEffect_BP OtherActor))
      (Default|ChangeMaterial _asprobe_effect_bp))))

(event EventTick
  (params (DeltaSeconds :type Float%20%28single-precision%29))
  (CallFunction|ActiveEngines)
  (bind _currentdelta (CallFunction|MirrorCooldown DeltaSeconds))
  (bind _currentdelta_2 (CallFunction|DecoyCooldown _currentdelta))
  (CallFunction|ProbeCooldown _currentdelta_2)
  (if (Variables|Default|Getdark)
    (Rendering|Components|Light|SetIntensity (Variables|Default|Getred) 2e+01)
    (Rendering|Components|Light|SetIntensity (Variables|Default|Getred2) 2e+01)
    (Rendering|Components|Light|SetIntensity (Variables|Default|GetEngine1) 0.0)
    (Rendering|Components|Light|SetIntensity (Variables|Default|GetEngine2) 0.0)
    (Rendering|Components|Light|SetIntensity (Variables|Default|GetEngine3) 0.0)
    (Rendering|Components|Light|SetIntensity (Variables|Default|GetEngine4) 0.0)
    (else
      (Rendering|Components|Light|SetIntensity (Variables|Default|Getred) 5e+02)
      (Rendering|Components|Light|SetIntensity (Variables|Default|Getred2) 5e+02)
      (Rendering|Components|Light|SetIntensity (Variables|Default|GetEngine1) 2e+01)
      (Rendering|Components|Light|SetIntensity (Variables|Default|GetEngine2) 2e+01)
      (Rendering|Components|Light|SetIntensity (Variables|Default|GetEngine3) 2e+01)
      (Rendering|Components|Light|SetIntensity (Variables|Default|GetEngine4) 2e+01))))

(event Input|ActionEvents|InputActionDeploy
  (params (Key :type Key%20Structure :default "AnyKey"))
  (:Pressed
    (bind _outactors (Actor|GetAllActorsOfClass "/Game/Blueprints/MirrorShot_BP.MirrorShot_BP_C"))
    (for _array_element _outactors
      (Default|DeployField _array_element))))

(fn ConstructionScript
  (Variables|Default|SetMirrorTimer (Variables|Default|GetMirrorCoolTime))
  (Variables|Default|SetDecoyTimer (Variables|Default|GetDecoyCoolTime))
  (Variables|Default|SetProbeTimer (Variables|Default|GetProbeCoolTime)))

(fn MirrorCooldown
  (params (TickDelta :type Float%20%28single-precision%29))
  (if (Variables|Default|GetmirrorOut)
    (if (<= (Variables|Default|GetMirrorTimer) 0.0)
      (Variables|Default|SetmirrorOut false)
      (Variables|Default|SetMirrorTimer (Variables|Default|GetMirrorCoolTime))
      (else
        (Variables|Default|SetMirrorTimer (- (Variables|Default|GetMirrorTimer) TickDelta)))))
  (return TickDelta))

(fn DecoyCooldown
  (params (TickDelta :type Float%20%28single-precision%29))
  (if (Variables|Default|GetdecoyOut)
    (if (<= (Variables|Default|GetDecoyTimer) 0.0)
      (Variables|Default|SetdecoyOut false)
      (Variables|Default|SetDecoyTimer (Variables|Default|GetDecoyCoolTime))
      (else
        (Variables|Default|SetDecoyTimer (- (Variables|Default|GetDecoyTimer) TickDelta)))))
  (return TickDelta))

(fn ProbeCooldown
  (params (TickDelta :type Float%20%28single-precision%29))
  (if (Variables|Default|GetprobeOut)
    (if (<= (Variables|Default|GetProbeTimer) 0.0)
      (Variables|Default|SetprobeOut false)
      (Variables|Default|SetProbeTimer (Variables|Default|GetProbeCoolTime))
      (else
        (Variables|Default|SetProbeTimer (- (Variables|Default|GetProbeTimer) TickDelta)))))
  (return TickDelta))

(fn ActiveEngines
  (bind _movementnumber (Variables|Default|GetmovementNumber))
  (if (or (Variables|Default|Getdark) (== _movementnumber 0.0))
    (Components|Activation|SetActive (Variables|Default|GetEngineSounds) false false)
    (Components|Activation|SetActive (Variables|Default|GetParticleSystem) false false)
    (Components|Activation|SetActive (Variables|Default|GetParticleSystem1) false false)
    (Components|Activation|SetActive (Variables|Default|GetParticleSystem2) false false)
    (Components|Activation|SetActive (Variables|Default|GetParticleSystem3) false false)
    (elif (< _movementnumber 0.0)
      (Components|Activation|SetActive (Variables|Default|GetEngineSounds) true false)
      (Components|Activation|SetActive (Variables|Default|GetParticleSystem) false false)
      (Components|Activation|SetActive (Variables|Default|GetParticleSystem1) false false)
      (Components|Activation|SetActive (Variables|Default|GetParticleSystem2) true false)
      (Components|Activation|SetActive (Variables|Default|GetParticleSystem3) true false)
      (elif (> _movementnumber 0.0)
        (Components|Activation|SetActive (Variables|Default|GetEngineSounds) true false)
        (Components|Activation|SetActive (Variables|Default|GetParticleSystem) true false)
        (Components|Activation|SetActive (Variables|Default|GetParticleSystem1) true false)
        (Components|Activation|SetActive (Variables|Default|GetParticleSystem2) false false)
        (Components|Activation|SetActive (Variables|Default|GetParticleSystem3) false false)))))